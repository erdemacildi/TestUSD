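; GM_Main is a test Blueprint for rendering USD stage sequences to images through Movie Render Queue.
; AddJob allocates one job, then for each USD stage actor sets its sequence and level, adds deferred, unlit and PNG settings with a short custom frame range.
; It starts a PIE executor render inside that loop.
; Nothing live calls AddJob: BeginPlay is empty, SetConfigs is a stub, and manifest-loading experiments are disconnected.
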(event `self.ReceiveBeginPlay`)

(fn `Add Job`
  (bind _returnvalue (`MoviePipelineQueue.AllocateNewJob` (`MoviePipelineQueueEngineSubsystem.GetQueue` (subsystem `MoviePipelineQueueEngineSubsystem`)) "/Script/MovieRenderPipelineCore.MoviePipelineExecutorJob"))
  ;[1 1 1] USD Stage Sequence
  (bind _outactors (`GameplayStatics.GetAllActorsOfClass` "/Script/USDStage.UsdStageActor"))
  (for _array_element _outactors
    (bind _returnvalue_2 (`UsdStageActor.GetLevelSequence` _array_element))
    (set `MoviePipelineExecutorJob.Sequence` (`KismetSystemLibrary.MakeSoftObjectPath` (`KismetSystemLibrary.GetSystemPath` _returnvalue_2)) _returnvalue)
    (set `MoviePipelineExecutorJob.Map` (`KismetSystemLibrary.MakeSoftObjectPath` (`KismetSystemLibrary.GetSystemPath` (`self.GetLevel`))) _returnvalue)
    (bind _returnvalue_3 (`MoviePipelineExecutorJob.GetConfiguration` _returnvalue))
    (`MoviePipelineConfigBase.FindOrAddSettingByClass` _returnvalue_3 "/Script/MovieRenderPipelineRenderPasses.MoviePipelineDeferredPassBase" false)
    (`MoviePipelineConfigBase.FindOrAddSettingByClass` _returnvalue_3 "/Script/MovieRenderPipelineRenderPasses.MoviePipelineDeferredPass_Unlit" false)
    (`MoviePipelineConfigBase.FindOrAddSettingByClass` _returnvalue_3 "/Script/MovieRenderPipelineRenderPasses.MoviePipelineImageSequenceOutput_PNG" false)
    (bind _returnvalue_4 (`MoviePipelineConfigBase.FindOrAddSettingByClass` _returnvalue_3 "/Script/MovieRenderPipelineCore.MoviePipelineOutputSetting" false))
    (set `MoviePipelineOutputSetting.CustomStartFrame` 1 _returnvalue_4)
    (set `MoviePipelineOutputSetting.CustomEndFrame` 11 _returnvalue_4)
    (`MoviePipelineQueueEngineSubsystem.RenderQueueWithExecutor` (subsystem `MoviePipelineQueueEngineSubsystem`) "/Script/MovieRenderPipelineEditor.MoviePipelinePIEExecutor")))

(fn `Set Configs`)

(fn `UserConstructionScript`)